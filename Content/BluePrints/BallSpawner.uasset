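; BallSpawner actor that places the single BP_GravityBall at its own location on BeginPlay and whenever RespawnBall is called.
; It reuses the first ball found in the level, otherwise spawns one behind a DoOnce.
; The ball is teleported with physics off and collision disabled, then collision returns after a short delay while physics simulation stays off.
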(event Custom|RespawnBall
  (bind _returnvalue (Transformation|GetActorLocation))
  (bind _outactors (Actor|GetAllActorsOfClass "/Game/BluePrints/BP_GravityBall.BP_GravityBall_C"))
  (Utilities|IsValid (Utilities|Array|Get(acopy) _outactors)
    (:Is%20Valid
      (bind _output_get (Variables|Default|SetBallRef (Utilities|Array|Get(acopy) _outactors))))
    (:Is%20Not%20Valid
      (Utilities|FlowControl|DoOnce false
        (:Completed
          (bind _returnvalue_2 (Game|SpawnActorfromClass "/Game/BluePrints/BP_GravityBall.BP_GravityBall_C" (Math|Transform|MakeTransform _returnvalue "0, 0, 0" "1,1,1") "AlwaysSpawn" 0 0))
          (Variables|Default|SetBallRef _returnvalue_2)))))
  (Physics|SetSimulatePhysics (Variables|/Game/BluePrints/BP_GravityBall.BP_GravityBall_C|GetCollisionComponent _output_get) false)
  (Transformation|SetActorLocation _output_get _returnvalue false true)
  (Collision|SetCollisionEnabled (Variables|/Game/BluePrints/BP_GravityBall.BP_GravityBall_C|GetCollisionComponent _output_get) "NoCollision")
  (Utilities|FlowControl|Delay 3.0)
  (Collision|SetCollisionEnabled (Variables|/Game/BluePrints/BP_GravityBall.BP_GravityBall_C|GetCollisionComponent _output_get) "QueryAndPhysics"))

(event EventBeginPlay
  (bind _returnvalue (Transformation|GetActorLocation))
  (bind _outactors (Actor|GetAllActorsOfClass "/Game/BluePrints/BP_GravityBall.BP_GravityBall_C"))
  (Utilities|IsValid (Utilities|Array|Get(acopy) _outactors)
    (:Is%20Valid
      (bind _output_get (Variables|Default|SetBallRef (Utilities|Array|Get(acopy) _outactors))))
    (:Is%20Not%20Valid
      (Utilities|FlowControl|DoOnce false
        (:Completed
          (bind _returnvalue_2 (Game|SpawnActorfromClass "/Game/BluePrints/BP_GravityBall.BP_GravityBall_C" (Math|Transform|MakeTransform _returnvalue "0, 0, 0" "1,1,1") "AlwaysSpawn" 0 0))
          (Variables|Default|SetBallRef _returnvalue_2)))))
  (Physics|SetSimulatePhysics (Variables|/Game/BluePrints/BP_GravityBall.BP_GravityBall_C|GetCollisionComponent _output_get) false)
  (Transformation|SetActorLocation _output_get _returnvalue false true)
  (Collision|SetCollisionEnabled (Variables|/Game/BluePrints/BP_GravityBall.BP_GravityBall_C|GetCollisionComponent _output_get) "NoCollision")
  (Utilities|FlowControl|Delay 3.0)
  (Collision|SetCollisionEnabled (Variables|/Game/BluePrints/BP_GravityBall.BP_GravityBall_C|GetCollisionComponent _output_get) "QueryAndPhysics"))

(fn ConstructionScript)