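; UberBall game mode that handles team assignment, player spawning and scoring for a two-team game.
; On login, NewPlayer tallies teams across GameplayPS player states and assigns the smaller team, favoring Team One on ties.
; Respawn spawns the requested class at a random PlayerStart, possesses it and applies team color, which new players' characters also receive.
; AddScore increments a team's score and copies both totals to GameplayGS.
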(event Custom|Respawn
  (params (TargetPC :type Controller%20Object%20Reference) (Class :type Uber%20Ball%20Character%20Class%20Reference))
  (bind _playerstate (Variables|/Script/Engine.Controller|GetPlayerState TargetPC))
  (bind _asgameplay_ps (Utilities|Casting|CastToGameplayPS _playerstate))
  (bind _team (Variables|/Game/BluePrints/GameplayPS.GameplayPS_C|GetTeam _asgameplay_ps))
  (bind _outactors (Actor|GetAllActorsOfClass "/Script/Engine.PlayerStart"))
  (if (Utilities|Enum|Equal(Enum) _team "NewEnumerator2")
    (CallFunction|NewPlayer TargetPC))
  (bind _returnvalue (Game|SpawnActorfromClass Class (Transformation|GetActorTransform (Utilities|Array|Get(acopy) _outactors (Math|Random|RandomIntegerinRange 0 (Utilities|Array|LastIndex _outactors)))) "AdjustIfPossibleButAlwaysSpawn" 0 _team 0))
  (Pawn|Possess TargetPC _returnvalue)
  (Default|SetTeamColour _returnvalue _team))

(event Custom|Add%20Score
  (params (Team :type TeamEnums%20Enum :default "NewEnumerator2"))
  (switch Utilities|FlowControl|Switch|SwitchonTeamEnums Team
    (:NewEnumerator0
      (bind _output_get (Variables|Default|SetTeam%201%20Score (+ (stale _output_get) 1))))
    (:NewEnumerator1
      (bind _output_get_2 (Variables|Default|SetTeam%202%20Score (+ (stale _output_get_2) 1)))))
  (bind _asgameplay_gs (Utilities|Casting|CastToGameplayGS (Game|GetGameState)))
  (Variables|/Game/BluePrints/Gameplay/GameplayGS.GameplayGS_C|SetTeam1Score _asgameplay_gs (Variables|Default|GetTeam%201%20Score))
  (Variables|/Game/BluePrints/Gameplay/GameplayGS.GameplayGS_C|SetTeam2Score _asgameplay_gs (Variables|Default|GetTeam%202%20Score)))

(event EventPostLogin
  (params (NewPlayer :type Player%20Controller%20Object%20Reference))
  (CallFunction|NewPlayer NewPlayer))

(event EventHandleStartingNewPlayer
  (params (NewPlayer :type Player%20Controller%20Object%20Reference))
  (|CallParentFunction NewPlayer)
  (bind _asuber_ball_character (Utilities|Casting|CastToUberBall_Character (Pawn|GetControlledPawn NewPlayer)))
  (Default|SetTeamColour _asuber_ball_character (Variables|/Game/BluePrints/GameplayPS.GameplayPS_C|GetTeam (.AsGameplay%20PS (Utilities|Casting|CastToGameplayPS (Variables|/Script/Engine.Controller|GetPlayerState NewPlayer))))))

(fn ConstructionScript)

(fn NewPlayer
  (params (New%20PLayer :type Controller%20Object%20Reference))
  (bind _playerstate (Variables|/Script/Engine.Controller|GetPlayerState New%20PLayer))
  (bind _outactors (Actor|GetAllActorsOfClass "/Game/BluePrints/GameplayPS.GameplayPS_C"))
  (for _array_element _outactors
    (|SetBy-RefVar (Utilities|Select :Index (Variables|/Game/BluePrints/GameplayPS.GameplayPS_C|GetTeam _array_element) :NewEnumerator2 (LocalVariables|GetTeam%20None) :NewEnumerator0 (LocalVariables|GetTeam1) :NewEnumerator1 (LocalVariables|GetTeam2)) (+ (Utilities|Select :Index (Variables|/Game/BluePrints/GameplayPS.GameplayPS_C|GetTeam _array_element) :NewEnumerator2 (LocalVariables|GetTeam%20None) :NewEnumerator0 (LocalVariables|GetTeam1) :NewEnumerator1 (LocalVariables|GetTeam2)) 1)))
  (if (> (LocalVariables|GetTeam1) (LocalVariables|GetTeam2))
    (bind _asgameplay_ps (Utilities|Casting|CastToGameplayPS _playerstate))
    (Variables|/Game/BluePrints/GameplayPS.GameplayPS_C|SetTeam _asgameplay_ps "NewEnumerator1")
    (else
      (bind _asgameplay_ps_2 (Utilities|Casting|CastToGameplayPS _playerstate))
      (Variables|/Game/BluePrints/GameplayPS.GameplayPS_C|SetTeam _asgameplay_ps_2 "NewEnumerator0"))))