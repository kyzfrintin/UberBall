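; BP_GravityBall is a ball that a ThirdPersonCharacter picks up on touch and loses when the ball is struck.
; An overlap while no player holds it calls AttachBallToPlayer on the character, which handles the attachment.
; A hit while held triggers a server event that detaches the ball, enables gravity, launches it along the scaled hit normal impulse as a velocity change, and clears the holder.
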(event OnComponentBeginOverlap(CollisionComponent)
  (params (OverlappedComponent :type Primitive%20Component%20Object%20Reference) (OtherActor :type Actor%20Object%20Reference) (OtherComp :type Primitive%20Component%20Object%20Reference) (OtherBodyIndex :type Integer) (bFromSweep :type Boolean) (SweepResult :type Hit%20Result%20Structure%20%28by%20ref%29))
  (Utilities|IsValid (Variables|Default|GetActiveParentPlayer)
    (:Is%20Not%20Valid
      (bind _asthird_person_character (Utilities|Casting|CastToThirdPersonCharacter OtherActor))
      (Default|AttachBalltoPlayer _asthird_person_character))))

(event OnComponentHit(CollisionComponent)
  (params (HitComponent :type Primitive%20Component%20Object%20Reference) (OtherActor :type Actor%20Object%20Reference) (OtherComp :type Primitive%20Component%20Object%20Reference) (NormalImpulse :type Vector :default "0, 0, 0") (Hit :type Hit%20Result%20Structure%20%28by%20ref%29))
  (Utilities|IsValid (Variables|Default|GetActiveParentPlayer)
    (:Is%20Valid
      (CallFunction|ServerHit NormalImpulse))))

(event Custom|Server_Hit
  (params (Normal%20Impulse :type Vector))
  (bind _collisioncomponent (Variables|Default|GetCollisionComponent))
  (Class|Actor|DetachRootComponentfromParent true)
  (Physics|SetEnableGravity _collisioncomponent true)
  (Physics|AddImpulse _collisioncomponent (* Normal%20Impulse 3e+02) "None" true)
  (Variables|Default|SetActiveParentPlayer 0))

(fn ConstructionScript)